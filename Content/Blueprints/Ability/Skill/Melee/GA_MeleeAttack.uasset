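; Gameplay ability for a melee attack that turns the avatar toward its combat target and plays a random tagged attack montage.
; When the montage's gameplay event arrives, it applies class-default damage to the target without a range or trace check.
; It then fires a MeleeImpact gameplay cue at the tagged combat socket, passing the montage tag, and ends.
; The ability also ends if the montage completes, is interrupted or is cancelled.
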(event `self.K2_ActivateAbility`
  (bind _returnvalue (`self.GetAvatarActorFromActorInfo`))
  (`self.K2_CommitAbility`)
  (set `self.HasHitTarget` false)
  (bind _returnvalue_2 (message `CombatInterface.GetCombatTarget` _returnvalue))
  (bind _output_get (set `self.CombatTarget` _returnvalue_2))
  (bind _ascombat_interface (cast `CombatInterface` _returnvalue))
  (`CombatInterface.UpdateFacingTarget` _ascombat_interface (`Actor.K2_GetActorLocation` _output_get))
  (bind _returnvalue_3 (message `CombatInterface.GetAttackMontages` (`self.GetAvatarActorFromActorInfo`)))
  (bind _output_get_2 (set `self.TaggedMontage` (`self.GetRandomTaggedMontageFromArray` _returnvalue_3)))
  (bind (_montage _montagetag _sockettag) (break `TaggedMontage` _output_get_2))
  (`AbilityTask_PlayMontageAndWait.CreatePlayMontageAndWaitProxy` "None" _montage
    (:`then`
      (`AbilityTask_WaitGameplayEvent.WaitGameplayEvent` _montagetag null
        (:`EventReceived`
          (bind _returnvalue_4 (message `CombatInterface.GetCombatSocketLocation` (`self.GetAvatarActorFromActorInfo`) _sockettag))
          (set `self.CombatSocketLocation` _returnvalue_4)
          (`TeamAbilitySystemLibrary.ApplyDamageEffect` (`self.MakeDamageEffectParamsFromClassDefaults` (`self.CombatTarget`)))
          (set `self.HasHitTarget` true)
          (bind _returnvalue_5 (message `CombatInterface.GetCombatTarget` (`self.GetAvatarActorFromActorInfo`)))
          (`self.K2_ExecuteGameplayCueWithParams` (struct :`TagName` "GameplayCue.MeleeImpact") (`AbilitySystemBlueprintLibrary.MakeGameplayCueParameters` 0.0 0.0 (struct) (struct) (struct) (`BlueprintGameplayTagLibrary.MakeGameplayTagContainerFromTag` (`.MontageTag` (break `TaggedMontage` (`self.TaggedMontage`)))) (struct) (`self.CombatSocketLocation`) (0.0 0.0 0.0) null (`self.GetAvatarActorFromActorInfo`) _returnvalue_5))
          (`self.K2_EndAbility`))))
    (:`OnCompleted`
      (`self.K2_EndAbility` :!label _label))
    (:`OnInterrupted`
      (goto _label))
    (:`OnCancelled`
      (goto _label))))